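; Player-controllable tank Blueprint that wires its components together and maps input to driving, camera aiming and firing.
; BeginPlay passes Barrel and Turret to their setters and initialises TankMovementComponent with both tracks.
; Driving works either through direct per-track throttle axes or through move and turn intents sent to TankMovementComponent.
; Aim axes rotate the azimuth gimbal and spring arm, while the Fire action calls Fire.
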(event `self.ReceiveBeginPlay`
  (`self.Setbarrelreference` (`self.Barrel`))
  (`self.SetTurretreference` (`self.Turret`))
  (`TankMovementComponent.Initialise` (`self.Tank Movement Component`) (`self.LeftTrack`) (`self.RightTrack`)))

(event `InputAxis|AimAzimuth`
  (params (AxisValue :type "Float (single-precision)"))
  ;[1 1 1] Aim InputBinding
  (`SceneComponent.K2_AddLocalRotation` (`self.Azimuth GImbal`) (`KismetMathLibrary.MakeRotator` 0.0 0.0 AxisValue) false false))

(event `InputAxis|LeftTrackThrottle`
  (params (AxisValue :type "Float (single-precision)"))
  ;[1 1 1] MOve input bind
  (`TankTrack.SetThrottle` (`self.LeftTrack`) AxisValue))

(event `InputAxis|RighTrackThrottle`
  (params (AxisValue :type "Float (single-precision)"))
  ;[1 1 1] MOve input bind
  (`TankTrack.SetThrottle` (`self.RightTrack`) AxisValue))

(event `InputAxis|AimElevation`
  (params (AxisValue :type "Float (single-precision)"))
  ;[1 1 1] Aim InputBinding
  (`SceneComponent.K2_AddLocalRotation` (`self.SpringArm`) (`KismetMathLibrary.MakeRotator` 0.0 AxisValue) false false))

(event `InputAxis|MoveForward`
  (params (AxisValue :type "Float (single-precision)"))
  ;[1 1 1] MOve input bind
  (`TankMovementComponent.IntentMoveForward` (`self.Tank Movement Component`) AxisValue))

(event `InputAction|Fire`
  (params (Key :type "Key Structure"))
  ;[1 1 1] Aim InputBinding
  (:`Pressed`
    (`self.Fire`)))

(event `InputAxis|MoveBackward`
  (params (AxisValue :type "Float (single-precision)"))
  ;[1 1 1] MOve input bind
  (`TankMovementComponent.IntentMoveForward` (`self.Tank Movement Component`) AxisValue))

(event `InputAxis|TurnRight`
  (params (AxisValue :type "Float (single-precision)"))
  ;[1 1 1] MOve input bind
  (`TankMovementComponent.TurnRight` (`self.Tank Movement Component`) AxisValue))

(event `InputAxis|TurnLeft`
  (params (AxisValue :type "Float (single-precision)"))
  ;[1 1 1] MOve input bind
  (`TankMovementComponent.TurnLeft` (`self.Tank Movement Component`) AxisValue))

(fn `UserConstructionScript`)